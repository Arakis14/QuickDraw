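; GM_Duel is the game mode for a samurai quick-draw duel between a player and an NPC.
; Tick moves the phase from Intro to Wait after the start time, then to Draw after a random delay, calling CallDrawPhaseStarted and showing the exclamation cue.
; AttackSuccesfully defeats the losing samurai and hides the cue, while SetGameFinished sets the Finish phase.
; BeginPlay finds both samurai and the cue actor by class.
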(event EventBeginPlay
  (bind _returnvalue (Actor|GetActorOfClass "/Game/BluePrints/BP_Exclamation.BP_Exclamation_C"))
  (Variables|Default|SetExclamationRef _returnvalue)
  (bind _returnvalue_2 (Actor|GetActorOfClass "/Game/BluePrints/BT_Samurai_Player.BT_Samurai_Player_C"))
  (Variables|Default|SetSamuraiPlayer _returnvalue_2)
  (bind _returnvalue_3 (Actor|GetActorOfClass "/Game/BluePrints/BT_Samurai_NPC.BT_Samurai_NPC_C"))
  (Variables|Default|SetSamuraiNPC _returnvalue_3))

(event EventTick
  (params (DeltaSeconds :type Float%20%28single-precision%29))
  (Variables|Default|SetElapsedTime (+ DeltaSeconds (Variables|Default|GetElapsedTime)))
  (switch Utilities|FlowControl|Switch|SwitchonE_Phase (Variables|Default|GetPhase)
    (:NewEnumerator0
      (if (>= (Variables|Default|GetElapsedTime) (Variables|Default|GetRoundStartTime))
        (Variables|Default|SetPhase "NewEnumerator1")
        (Utilities|FlowControl|Delay (Math|Random|RandomFloatinRange (Variables|Default|GetMinDrawDelay) (Variables|Default|GetMaxDrawDelay)))
        (Variables|Default|SetPhase "NewEnumerator2")
        (Default|CallDrawPhaseStarted)
        (Utilities|IsValid (Variables|Default|GetExclamationRef)
          (:Is%20Valid
            (Default|SetVisibility (Variables|Default|GetExclamationRef) true))
          (:Is%20Not%20Valid
            (Development|PrintString "Exclamation not found!")))))))

(fn ConstructionScript)

(fn SetGameFinished
  (Variables|Default|SetPhase "NewEnumerator3"))

(fn AttackSuccesfully
  (params (isPlayer :type Boolean))
  (if isPlayer
    (Default|Defeated (Variables|Default|GetSamuraiNPC))
    (else
      (Default|Defeated (Variables|Default|GetSamuraiPlayer))))
  (Utilities|IsValid (Variables|Default|GetExclamationRef)
    (:Is%20Valid
      (Default|SetVisibility (Variables|Default|GetExclamationRef) false))))